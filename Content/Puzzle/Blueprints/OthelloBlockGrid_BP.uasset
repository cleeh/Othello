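; Othello board that serves as a TensorFlow reinforcement-learning environment, pitting the AI as White against random-move Black.
; It sends state, reward and legal-move mask as JSON, then plays the returned cell index.
; Rewards scale with flipped stones plus win/loss bonuses; game over starts training, whose completion resets the board.
; G triggers a Black auto-move; F toggles running it every Tick.
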(event OnInputResults(TensorflowComponent)
  (params (Results :type String))
  (bind _returnvalue (Math|Conversions|ToInteger(Byte) Results))
  (bind _size (Variables|Default|GetSize))
  (bind _returnvalue_2 (/ _returnvalue _size))
  (bind _returnvalue_3 (Math|Integer|%(Integer) _returnvalue _size))
  ;[1 1 1] AI Process
  (if (>= (Math|Conversions|ToInteger(Byte) Results) 0)
    (CallFunction|ResetReward)
    (bind _returnvalue_4 (Class|OthelloBlockGrid|GetBlock _returnvalue_3 _returnvalue_2))
    (bind _returnvalue_5 (Class|OthelloBlock|PutStone _returnvalue_4))
    (if _returnvalue_5
      (bind _returnvalue_6 (Class|OthelloBlockGrid|ChangeStonesColor (Math|Conversions|ToByte(Integer) _returnvalue_3) (Math|Conversions|ToByte(Integer) _returnvalue_2)))
      (CallFunction|AddReward (* _returnvalue_6 (Variables|Reward|GetConst%20White%20Get%20Reward)))
      (CallFunction|CheckOverandOmit)
      (else
        (Development|PrintString "# [Error!] Putting Stone #")))))

(event OnTrainingComplete(TensorflowComponent)
  (params (SummaryJson :type String))
  ;[1 1 1] 게임이 끝나면 훈련 시작
  (Class|OthelloGameMode|GameOver (.AsOthello%20Game%20Mode (Utilities|Casting|CastToOthelloGameMode (Game|GetGameMode))))
  (Class|OthelloBlockGrid|ResetGrid))

(event EventBeginPlay
  (Input|EnableInput (Game|GetPlayerController 0)))

(event EventTick
  (params (DeltaSeconds :type Float%20%28single-precision%29))
  (bind _size (Variables|Default|GetSize))
  ;[1 1 1] 게임 진행 자동화
  (if (Variables|Default|GetIterator)
    (bind _changednumber (CallFunction|PutStoneAuto))
    (CallFunction|AddReward (* _changednumber (Variables|Reward|GetConst%20Black%20Get%20Penalty)))
    (Variables|Default|SetShouldOmit true)
    (Class|OthelloBlockGrid|UpdatePutablePosition)
    (for _index (range 0 (- (* _size _size) 1))
      (if (Utilities|Array|Get(acopy) (Variables|Default|GetIsPutable) _index)
        (Variables|Default|SetShouldOmit false)
        (CallFunction|CheckOverandOmit)))
    (if (not (Variables|Default|GetShouldOmit))
      (CallFunction|SendState (Variables|Reward|GetReward%20Total)))))

(event EventAfterPutStoneBlack
  (bind _size (Variables|Default|GetSize))
  (Variables|Default|SetShouldOmit true)
  (Class|OthelloBlockGrid|UpdatePutablePosition)
  (for _index (range 0 (- (* _size _size) 1))
    (if (Utilities|Array|Get(acopy) (Variables|Default|GetIsPutable) _index)
      (Variables|Default|SetShouldOmit false)
      (CallFunction|CheckOverandOmit)))
  (if (not (Variables|Default|GetShouldOmit))
    (CallFunction|SendState (Variables|Reward|GetReward%20Total))))

(event Input|KeyboardEvents|G
  (params (Key :type Key%20Structure))
  (bind _size (Variables|Default|GetSize))
  (:Pressed
    ;[1 1 1] 게임 진행 자동화
    (bind _changednumber (CallFunction|PutStoneAuto))
    (CallFunction|AddReward (* _changednumber (Variables|Reward|GetConst%20Black%20Get%20Penalty)))
    (Variables|Default|SetShouldOmit true)
    (Class|OthelloBlockGrid|UpdatePutablePosition)
    (for _index (range 0 (- (* _size _size) 1))
      (if (Utilities|Array|Get(acopy) (Variables|Default|GetIsPutable) _index)
        (Variables|Default|SetShouldOmit false)
        (CallFunction|CheckOverandOmit)))
    (if (not (Variables|Default|GetShouldOmit))
      (CallFunction|SendState (Variables|Reward|GetReward%20Total)))))

(event Input|KeyboardEvents|F
  (params (Key :type Key%20Structure))
  ;[1 1 1] 게임 진행 자동화
  (:Pressed
    (Variables|Default|SetIterator (not (Variables|Default|GetIterator)))))

(fn ConstructionScript)

(fn SendState
  (params (Reward :type Float%20%28single-precision%29))
  (Class|OthelloBlockGrid|UpdatePutablePosition)
  (Default|SendJsonInput (Variables|Default|GetTensorflowComponent) (Class|SIOJsonObject|EncodeJson (Class|SIOJLibrary|StructtoJsonObject (Utilities|Struct|MakeTrainStruct (Class|OthelloBlockGrid|GetState) Reward (Class|OthelloBlockGrid|IsGameOver) (Variables|Default|GetIsPutable))))))

(fn PutStoneAuto
  (bind _putablearray (LocalVariables|GetPutableArray))
  (bind _size (Variables|Default|GetSize))
  (bind _size_2 (Variables|Default|GetSize))
  (bind _putablearray_2 (LocalVariables|GetPutableArray))
  (bind _returnvalue (Utilities|Array|Length _putablearray))
  (bind _returnvalue_2 (Math|Random|RandomInteger _returnvalue))
  (bind _output (Utilities|Array|Get(acopy) _putablearray_2 _returnvalue_2))
  (Utilities|FlowControl|Sequence
    (:then_0
      (Class|OthelloBlockGrid|UpdatePutablePosition)
      (for _index (range 0 (- (* _size_2 _size_2) 1))
        (if (Utilities|Array|Get(acopy) (Variables|Default|GetIsPutable) _index)
          (Utilities|Array|Add (LocalVariables|GetPutableArray) _index))))
    (:then_1
      (if (> _returnvalue 0)
        (bind _returnvalue_3 (Class|OthelloBlockGrid|GetBlock (Math|Integer|%(Integer) _output _size) (/ _output _size)))
        (bind _returnvalue_4 (Class|OthelloBlock|PutStone _returnvalue_3))
        (if _returnvalue_4
          (bind _returnvalue_5 (Class|OthelloBlockGrid|ChangeStonesColor (Math|Conversions|ToByte(Integer) (Variables|/Script/Othello.OthelloBlock|GetX _returnvalue_3)) (Math|Conversions|ToByte(Integer) (Variables|/Script/Othello.OthelloBlock|GetY _returnvalue_3))))
          (return _returnvalue_5)
          (else
            (Development|PrintString "[Auto] Puting stone fail")))
        (else
          (CallFunction|CheckOverandOmit))))))

(fn AddReward
  (params (NewParam :type Float%20%28single-precision%29))
  (Variables|Reward|SetReward%20Total (+ NewParam (Variables|Reward|GetReward%20Total))))

(fn ResetReward
  (Variables|Reward|SetReward%20Total 0.0))

(fn CheckOverandOmit
  ;[1 1 1] 게임이 종료/차례 넘김 판별, 승리자 보상
  (bind _returnvalue (Class|OthelloBlockGrid|CheckGameOver))
  (if _returnvalue
    (bind _returnvalue_2 (Class|OthelloBlockGrid|WhatColorIsMore))
    (switch Utilities|FlowControl|Switch|SwitchonEStoneColor _returnvalue_2
      (:None
        (Development|PrintString "Draw!"))
      (:Black
        (CallFunction|AddReward (Variables|Reward|GetConst%20Black%20Win%20Penalty))
        (Development|PrintString "Black Wins~!"))
      (:White
        (CallFunction|AddReward (Variables|Reward|GetConst%20White%20Win%20Reward))
        (Development|PrintString "White Wins~!")))
    (CallFunction|SendState (Variables|Reward|GetReward%20Total))
    (Default|BeginTraining (Variables|Default|GetTensorflowComponent))))